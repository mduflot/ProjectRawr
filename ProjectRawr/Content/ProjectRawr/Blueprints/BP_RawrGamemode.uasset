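; Game mode for ProjectRawr that spawns players as BP_RawrCharacter at one of two tagged PlayerStarts.
; On server PostLogin, it caches the Player1 start and the other start, calling ClientPostLogin on the joining BP_RawrController when it finds Player1.
; SpawnPlayerEvent replaces a controller's existing pawn and possesses the new character.
; The first PlayerArray entry gets the Player1 start; everyone else gets the second.
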(event Custom|SpawnPlayerEvent
  (params (Player%20Controller :type Player%20Controller%20Object%20Reference))
  (bind _returnvalue (Pawn|GetControlledPawn Player%20Controller))
  ;[1 1 1] Spawn Player At Proper Location
  (Utilities|IsValid _returnvalue
    (:Is%20Valid
      (Actor|DestroyActor _returnvalue)
      (if (== (Variables|/Script/Engine.PlayerState|GetPlayerId (Variables|/Script/Engine.Controller|GetPlayerState Player%20Controller)) (Variables|/Script/Engine.PlayerState|GetPlayerId (Utilities|Array|Get(acopy) (Variables|/Script/Engine.GameStateBase|GetPlayerArray (Game|GetGameState)))))
        (bind _returnvalue_2 (Game|SpawnActorfromClass "/Game/ProjectRawr/Characters/BP_RawrCharacter.BP_RawrCharacter_C" (Transformation|GetActorTransform (Variables|Default|GetSpawn1)) "AdjustIfPossibleButDontSpawnIfColliding" "MultiplyWithRoot" 0 0))
        (Pawn|Possess Player%20Controller _returnvalue_2)
        (else
          (bind _returnvalue_3 (Game|SpawnActorfromClass "/Game/ProjectRawr/Characters/BP_RawrCharacter.BP_RawrCharacter_C" (Transformation|GetActorTransform (Variables|Default|GetSpawn2)) "AdjustIfPossibleButDontSpawnIfColliding" "MultiplyWithRoot" 0 0))
          (Pawn|Possess Player%20Controller _returnvalue_3))))))

(event EventPostLogin
  (params (NewPlayer :type Player%20Controller%20Object%20Reference))
  ;[1 1 1] Player Spawn Initialization
  (Networking|SwitchHasAuthority
    (:Authority
      (bind _outactors (Actor|GetAllActorsOfClass "/Script/Engine.PlayerStart"))
      (for _array_element _outactors
        (if (== (Variables|/Script/Engine.PlayerStart|GetPlayerStartTag _array_element) "Player1")
          (Variables|Default|SetSpawn1 _array_element)
          (bind _asbp_rawr_controller (Utilities|Casting|CastToBP_RawrController NewPlayer))
          (Default|ClientPostLogin _asbp_rawr_controller)
          (else
            (Variables|Default|SetSpawn2 _array_element)))))))

(fn ConstructionScript)