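; BP_Monster is an enemy that feeds its AI blackboard an end location and a nearby target.
; On BeginPlay it writes a zero-vector end location to the blackboard.
; Sphere2 overlap events add or remove Interface_Health actors in a list, then run SetTarget.
; SetTarget switches the blackboard target to any listed actor closer than the current one, without clearing targets that leave the sphere.
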(event OnComponentBeginOverlap(Sphere2)
  (params (OverlappedComponent :type Primitive%20Component%20Object%20Reference) (OtherActor :type Actor%20Object%20Reference) (OtherComp :type Primitive%20Component%20Object%20Reference) (OtherBodyIndex :type Integer) (bFromSweep :type Boolean) (SweepResult :type Hit%20Result%20Structure%20%28by%20ref%29))
  ;[1 1 1] Check Enemies around
  (if (Utilities|DoesObjectImplementInterface OtherActor "/Script/ProjectRawr.Interface_Health")
    (Utilities|Array|Add (Variables|Default|GetActors) OtherActor)
    (CallFunction|SetTarget)))

(event OnComponentEndOverlap(Sphere2)
  (params (OverlappedComponent :type Primitive%20Component%20Object%20Reference) (OtherActor :type Actor%20Object%20Reference) (OtherComp :type Primitive%20Component%20Object%20Reference) (OtherBodyIndex :type Integer))
  ;[1 1 1] Check Enemies around
  (if (Utilities|DoesObjectImplementInterface OtherActor "/Script/ProjectRawr.Interface_Health")
    (Utilities|Array|RemoveItem (Variables|Default|GetActors) OtherActor)
    (CallFunction|SetTarget)))

(event Custom|SetTarget
  (bind _returnvalue (AI|GetBlackboard 0))
  (bind _blackboardkeytarget (Variables|Default|GetBlackboardKeyTarget))
  (bind _returnvalue_2 (AI|Components|Blackboard|GetValueasObject _returnvalue _blackboardkeytarget))
  ;[1 1 1] SetTarget
  (for _array_element (Variables|Default|GetActors)
    (if (Utilities|IsValid _returnvalue_2)
      (if (> (Math|Vector|Distance(Vector) (Transformation|GetActorLocation (.AsActor (Utilities|Casting|CastToActor _returnvalue_2))) (Transformation|GetActorLocation)) (Math|Vector|Distance(Vector) (Transformation|GetActorLocation (.AsActor (Utilities|Casting|CastToActor _array_element))) (Transformation|GetActorLocation)))
        (AI|Components|Blackboard|SetValueasObject (AI|GetBlackboard 0) (Variables|Default|GetBlackboardKeyTarget) _array_element))
      (else
        (AI|Components|Blackboard|SetValueasObject (AI|GetBlackboard 0) (Variables|Default|GetBlackboardKeyTarget) _array_element)))))

(event EventBeginPlay
  ;[1 1 1] Set EndLocation at BeginPlay
  (if true
    (Variables|Default|SetEndLocation "0, 0, 0")
    (else
      (Variables|Default|SetEndLocation "0, 0, 0")))
  (AI|Components|Blackboard|SetValueasVector (AI|GetBlackboard 0) (Variables|Default|GetBlackboardKeyEndLocation) (Variables|Default|GetEndLocation)))

(fn ConstructionScript)