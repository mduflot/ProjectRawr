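; Character Blueprint for Project Rawr that lets the player request an enemy spawn through Enhanced Input.
; Pressing IA_Spawn calls SpawnMyEnemyOnServer, which casts the game mode to BP_RawrGamemode and passes this character to its ServerSpawnEnemy.
; HitReaction and GetHealth overrides only forward to the parent class, and BeginPlay and the construction script are empty.
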(event Custom|SpawnMyEnemyOnServer
  (Default|ServerSpawnEnemy (.AsBP%20Rawr%20Gamemode (Utilities|Casting|CastToBP_RawrGamemode (Game|GetGameMode))) self))

(event Input|EnhancedActionEvents|EnhancedInputActionIA_Spawn
  (params (ActionValue :type Boolean) (ElapsedSeconds :type Float%20%28double-precision%29) (TriggeredSeconds :type Float%20%28double-precision%29) (InputAction :type Input%20Action%20Object%20Reference :default "/Game/ProjectRawr/Characters/Input/Actions/IA_Spawn.IA_Spawn"))
  (:Started
    (CallFunction|SpawnMyEnemyonServer)))

(event EventBeginPlay)

(event EventHitReaction
  (|CallParentFunction))

(fn ConstructionScript)

(fn GetHealth
  (bind _returnvalue (|CallParentFunction))
  (return _returnvalue))