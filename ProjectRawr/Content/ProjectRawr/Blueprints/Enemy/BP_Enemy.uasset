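; BP_Enemy is an enemy actor with health, a floating health bar and a detection sphere.
; Each HitReaction removes one health point, prints a debug message, updates the WBP_EnemyHUD bar and destroys the actor at zero.
; The widget turns toward the player camera every Tick.
; SphereDetection tracks overlapping Interface_Health actors in an Actors array, which nothing here reads beyond its removal check.
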(event OnComponentBeginOverlap(SphereDetection)
  (params (OverlappedComponent :type Primitive%20Component%20Object%20Reference) (OtherActor :type Actor%20Object%20Reference) (OtherComp :type Primitive%20Component%20Object%20Reference) (OtherBodyIndex :type Integer) (bFromSweep :type Boolean) (SweepResult :type Hit%20Result%20Structure%20%28by%20ref%29))
  (if (Utilities|DoesObjectImplementInterface OtherActor "/Script/ProjectRawr.Interface_Health")
    (Utilities|Array|Add (Variables|Default|GetActors) OtherActor)))

(event OnComponentEndOverlap(SphereDetection)
  (params (OverlappedComponent :type Primitive%20Component%20Object%20Reference) (OtherActor :type Actor%20Object%20Reference) (OtherComp :type Primitive%20Component%20Object%20Reference) (OtherBodyIndex :type Integer))
  (if (Utilities|Array|ContainsItem (Variables|Default|GetActors) OtherActor)
    (Utilities|Array|RemoveItem (Variables|Default|GetActors) OtherActor)))

(event EventTick
  (params (DeltaSeconds :type Float%20%28single-precision%29))
  (Transformation|SetWorldRotation (Variables|Default|GetWidget) (Math|Rotator|FindLookatRotation (Transformation|GetWorldLocation (Variables|Default|GetWidget)) (Transformation|GetWorldLocation (Variables|/Script/Engine.PlayerCameraManager|GetTransformComponent (Game|GetPlayerCameraManager 0)))) false false))

(event EventBeginPlay
  (Default|UpdateHealth (.AsWBP%20Enemy%20HUD (Utilities|Casting|CastToWBP_EnemyHUD (UserInterface|GetUserWidgetObject (Variables|Default|GetWidget)))) (/ (Variables|Default|GetHealth) (Variables|Default|GetMaxHealth))))

(event EventHitReaction
  (bind _result (Math|Integer|DecrementInt (Variables|Default|GetHealth))
    (:%20%20
      (Development|PrintString "Hit reaction!")
      (Default|UpdateHealth (.AsWBP%20Enemy%20HUD (Utilities|Casting|CastToWBP_EnemyHUD (UserInterface|GetUserWidgetObject (Variables|Default|GetWidget)))) (/ _result (Variables|Default|GetMaxHealth)))
      (if (<= _result 0)
        (Actor|DestroyActor)))))

(fn ConstructionScript)

(fn GetHealth
  (return (Variables|Default|GetHealth)))